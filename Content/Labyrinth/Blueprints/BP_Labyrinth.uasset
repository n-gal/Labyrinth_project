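; Labyrinth actor that generates a maze on a tile grid using randomized depth-first search with backtracking, animated as a debug visualization.
; The construction script fills the tile array and spawns floor instances on one HISM.
; From BeginPlay, half-second steps pick seeded random unvisited neighbors or pop the stack, coloring tiles through per-instance custom data.
; Wall removal only updates tile data, as DrawWall is an uncalled stub.
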(event EventBeginPlay
  (bind _completed (CallFunction|GotoRandomNeighbor (Variables|Default|GetcurrentTileIndex) :!label _label))
  (if _completed
    (Development|PrintString "Maze completed")
    (else
      (Utilities|FlowControl|Delay 0.5)
      (goto _label))))

(event Collision|EventActorBeginOverlap
  (params (OtherActor :type Actor%20Object%20Reference)))

(event EventTick
  (params (DeltaSeconds :type Float%20%28single-precision%29)))

(fn ConstructionScript
  (Components|InstancedStaticMesh|ClearInstances (Variables|Default|GetHierarchicalInstancedStaticMesh))
  (Utilities|Array|Clear (Variables|Default|Gettiles))
  (Rendering|Material|CreateDynamicMaterialInstance (Variables|Default|GetHierarchicalInstancedStaticMesh) 0 "/Game/Labyrinth/Materials/M_DebugLabyrinthFloor.M_DebugLabyrinthFloor" "None" :!class /Script/Engine.PrimitiveComponent)
  (for _index (range 0 (- (Variables|Default|GetrowCount) 1))
    (for _index_2 (range 0 (- (Variables|Default|GetcolCount) 1))
      (bind _returnvalue (Utilities|Array|Add (Variables|Default|Gettiles) (Utilities|Struct|MakeS_Tile (Variables|Default|GettileMesh) false _index _index_2 (Variables|Default|GettileMeshSize) true true true true 0)))
      (CallFunction|DrawTile (Utilities|Array|Get(acopy) (Variables|Default|Gettiles) _returnvalue)))))

(fn DrawTile
  (params (S_Tile :type S%20Tile%20Structure%20%28by%20ref%29))
  (bind (_tilemesh _row _col _size) (Utilities|Struct|BreakS_Tile S_Tile))
  (bind _mazesize (Variables|Default|GetmazeSize))
  (bind _hierarchicalinstancedstaticmesh (Variables|Default|GetHierarchicalInstancedStaticMesh))
  (bind _returnvalue (* _size _mazesize))
  (Components|StaticMesh|SetStaticMesh _hierarchicalinstancedstaticmesh _tilemesh)
  (bind _returnvalue_2 (Components|InstancedStaticMesh|AddInstance _hierarchicalinstancedstaticmesh (Math|Transform|MakeTransform (Math|Vector|MakeVector (* _row _returnvalue) (* _col _returnvalue) 0.0) "0, 0, 0" (Math|Conversions|ToVector(Float) _mazesize)) false))
  (CallFunction|SetTileColor _returnvalue_2 "(R=1.000000,G=1.000000,B=1.000000,A=1.000000)"))

(fn GetIndex
  (params (TileRow :type Integer) (TileCol :type Integer))
  (bind _isvalid (CallFunction|IsNeighborValid TileRow TileCol))
  (if _isvalid
    (return (+ TileCol (* TileRow (Variables|Default|GetcolCount))))
    (else
      (return -1))))

(fn CheckNeighbors
  (params (Tile :type S%20Tile%20Structure))
  (bind (_row _col) (Utilities|Struct|BreakS_Tile Tile))
  (bind (_row_2 _col_2) (Utilities|Struct|BreakS_Tile Tile))
  (bind (_row_3 _col_3) (Utilities|Struct|BreakS_Tile Tile))
  (bind (_row_4 _col_4) (Utilities|Struct|BreakS_Tile Tile))
  (Utilities|FlowControl|Sequence
    (:then_0
      (bind _tile (CallFunction|GetTile _row_2 (- _col_2 1)))
      (LocalVariables|Settop _tile))
    (:then_1
      (bind _tile_2 (CallFunction|GetTile (+ _row_3 1) _col_3))
      (LocalVariables|Setright _tile_2))
    (:then_2
      (bind _tile_3 (CallFunction|GetTile _row_4 (+ _col_4 1)))
      (LocalVariables|Setbottom _tile_3))
    (:then_3
      (bind _tile_4 (CallFunction|GetTile (- _row 1) _col))
      (LocalVariables|Setleft _tile_4))
    (:then_4
      (Utilities|FlowControl|Sequence
        (:then_0
          (if (not (.isVisited (Utilities|Struct|BreakS_Tile (LocalVariables|Gettop))))
            (bind _index (CallFunction|GetIndex (.row (Utilities|Struct|BreakS_Tile (LocalVariables|Gettop))) (.col (Utilities|Struct|BreakS_Tile (LocalVariables|Gettop)))))
            (Utilities|Array|Add (LocalVariables|Getneighbors) _index)))
        (:then_1
          (if (not (.isVisited (Utilities|Struct|BreakS_Tile (LocalVariables|Getright))))
            (bind _index_2 (CallFunction|GetIndex (.row (Utilities|Struct|BreakS_Tile (LocalVariables|Getright))) (.col (Utilities|Struct|BreakS_Tile (LocalVariables|Getright)))))
            (Utilities|Array|Add (LocalVariables|Getneighbors) _index_2)))
        (:then_2
          (if (not (.isVisited (Utilities|Struct|BreakS_Tile (LocalVariables|Getbottom))))
            (bind _index_3 (CallFunction|GetIndex (.row (Utilities|Struct|BreakS_Tile (LocalVariables|Getbottom))) (.col (Utilities|Struct|BreakS_Tile (LocalVariables|Getbottom)))))
            (Utilities|Array|Add (LocalVariables|Getneighbors) _index_3)))
        (:then_3
          (if (not (.isVisited (Utilities|Struct|BreakS_Tile (LocalVariables|Getleft))))
            (bind _index_4 (CallFunction|GetIndex (.row (Utilities|Struct|BreakS_Tile (LocalVariables|Getleft))) (.col (Utilities|Struct|BreakS_Tile (LocalVariables|Getleft)))))
            (Utilities|Array|Add (LocalVariables|Getneighbors) _index_4))
          (return (LocalVariables|Getneighbors)))))))

(fn GetTile
  (params (TileRow :type Integer) (TileCol :type Integer))
  (bind _index (CallFunction|GetIndex TileRow TileCol))
  (if (!= _index -1)
    (return (Utilities|Array|Get(acopy) (Variables|Default|Gettiles) _index))
    (else
      (return (Utilities|Struct|MakeS_Tile true)))))

(fn IsNeighborValid
  (params (TileRow :type Integer) (TileCol :type Integer))
  (return (not (or (or (< TileRow 0) (< TileCol 0)) (or (> TileRow (- (Variables|Default|GetrowCount) 1)) (> TileCol (- (Variables|Default|GetcolCount) 1)))))))

(fn GotoRandomNeighbor
  (params (StartingTileIndex :type Integer))
  (bind _stack (Variables|Default|Getstack))
  (bind _tiles (Variables|Default|Gettiles))
  (bind _stack_2 (Variables|Default|Getstack))
  (bind _tiles_2 (Variables|Default|Gettiles))
  (bind _output (Utilities|Array|Get(acopy) _tiles_2 StartingTileIndex))
  (bind (_row _col) (Utilities|Struct|BreakS_Tile _output))
  (CallFunction|SetTileColor StartingTileIndex "(R=1.000000,G=0.037924,B=0.000000,A=1.000000)")
  (Utilities|Struct|SetmembersinS_Tile _output true)
  (bind _unvisitedneighbors (CallFunction|CheckNeighbors _output))
  (bind _output_get (LocalVariables|SetavailableNeighbors _unvisitedneighbors))
  (if (> (Utilities|Array|Length _output_get) 0)
    (LocalVariables|SetNextTileIndex (Utilities|Array|Get(acopy) (LocalVariables|GetavailableNeighbors) (Math|Random|RandomIntegerinRangefromStream (Math|Random|MakeRandomStream (* (Variables|Default|Getseed) _row _col)) 0 (- (Utilities|Array|Length (LocalVariables|GetavailableNeighbors)) 1))))
    (bind (_newcurcell _newnextcell) (CallFunction|RemoveWalls (Variables|Default|GetcurrentTileIndex) (LocalVariables|GetNextTileIndex)))
    (Utilities|Array|SetArrayElem _tiles (Variables|Default|GetcurrentTileIndex) _newcurcell)
    (Utilities|Array|SetArrayElem _tiles (LocalVariables|GetNextTileIndex) _newnextcell)
    (bind _output_get_2 (Variables|Default|SetcurrentTileIndex (LocalVariables|GetNextTileIndex)))
    (Utilities|Array|Add (Variables|Default|Getstack) _output_get_2)
    (CallFunction|SetTileColor _output_get_2 "(R=1.000000,G=0.000000,B=0.833106,A=1.000000)")
    (return false)
    (elif (> (Utilities|Array|Length _stack) 0)
      (Utilities|Array|RemoveIndex _stack_2 (Utilities|Array|LastIndex _stack))
      (bind _lastcellindex (CallFunction|GetLastValue _stack_2))
      (bind _output_get_3 (Variables|Default|SetcurrentTileIndex _lastcellindex))
      (CallFunction|SetTileColor _output_get_3 "(R=1.000000,G=0.000000,B=0.833106,A=1.000000)")
      (return false)
      (else
        (return true)))))

(fn DebugPrintTilePos
  (params (TileIndex :type Integer))
  (bind _tiles (Variables|Default|Gettiles))
  (bind _output (Utilities|Array|Get(acopy) _tiles TileIndex))
  (Development|PrintString (Utilities|String|Append (Utilities|String|ToString(Integer) (.row _output)) "   " (Utilities|String|ToString(Integer) (.col _output)))))

(fn DebugSetTileColor
  (params (TileIndex :type Integer)))

(fn SetTileColor
  (params (Instance%20Index :type Integer) (New%20Color :type Linear%20Color%20Structure))
  (bind _hierarchicalinstancedstaticmesh (Variables|Default|GetHierarchicalInstancedStaticMesh))
  (Components|InstancedStaticMesh|SetCustomDataValue _hierarchicalinstancedstaticmesh Instance%20Index 0 (.r New%20Color) false)
  (Components|InstancedStaticMesh|SetCustomDataValue _hierarchicalinstancedstaticmesh Instance%20Index 1 (.g New%20Color) false)
  (Components|InstancedStaticMesh|SetCustomDataValue _hierarchicalinstancedstaticmesh Instance%20Index 2 (.b New%20Color) false))

(fn GetLastValue
  (params (List :type Array%20of%20Integers))
  (if (<= (Utilities|Array|Length List) 0)
    (return 0)
    (else
      (return (Utilities|Array|Get(acopy) List (Utilities|Array|LastIndex List))))))

(fn RemoveWalls
  (params (CurCellIndex :type Integer) (NextCellIndex :type Integer))
  (bind _tiles (Variables|Default|Gettiles))
  (bind _output (Utilities|Array|Get(acopy) _tiles NextCellIndex))
  (bind _output_2 (Utilities|Array|Get(acopy) _tiles CurCellIndex))
  (bind (_row _col) (Utilities|Struct|BreakS_Tile _output))
  (bind (_row_2 _col_2) (Utilities|Struct|BreakS_Tile _output_2))
  (LocalVariables|SetModifCurCell _output_2)
  (LocalVariables|SetModifNextCell _output)
  (Utilities|FlowControl|Sequence
    (:then_0
      (bind _output_get (LocalVariables|Setx (- _col_2 _col)))
      (if (== _output_get 1)
        (Utilities|Struct|SetmembersinS_Tile (LocalVariables|GetModifCurCell) false)
        (Utilities|Struct|SetmembersinS_Tile (LocalVariables|GetModifNextCell) false)
        (Development|PrintString "Vertical Movement" :!label _label)
        (elif (== _output_get -1)
          (Utilities|Struct|SetmembersinS_Tile (LocalVariables|GetModifCurCell) false)
          (Utilities|Struct|SetmembersinS_Tile (LocalVariables|GetModifNextCell) false)
          (goto _label))))
    (:then_1
      (bind _output_get_2 (LocalVariables|Sety (- _row_2 _row)))
      (if (== _output_get_2 1)
        (Utilities|Struct|SetmembersinS_Tile (LocalVariables|GetModifCurCell) false)
        (Utilities|Struct|SetmembersinS_Tile (LocalVariables|GetModifNextCell) false)
        (Development|PrintString "Horizontal  Movement")
        (elif (== _output_get_2 -1)
          (Utilities|Struct|SetmembersinS_Tile (LocalVariables|GetModifCurCell) false)
          (Utilities|Struct|SetmembersinS_Tile (LocalVariables|GetModifNextCell) false)
          (Development|PrintString "Horizontal  Movement")
          (else
            (return (LocalVariables|GetModifCurCell) (LocalVariables|GetModifNextCell)))))
      (return (LocalVariables|GetModifCurCell) (LocalVariables|GetModifNextCell)))))

(fn DrawWall
  (params (TileIndex :type Integer))
  (Components|StaticMesh|SetStaticMesh (Variables|Default|GetHierarchicalInstancedStaticMesh) (Variables|Default|GetwallMesh)))